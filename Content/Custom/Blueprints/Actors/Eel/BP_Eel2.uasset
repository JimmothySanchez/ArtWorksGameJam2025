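; BP_Eel2 is an eel actor with a floating pawn movement component, a swimming head motion and periodic bubble effects.
; A timeline sets HeadLocation from its head track scaled by speed relative to max, and NormalizedElasticity inversely from the mesh's physics angular velocity, printing the latter for debugging.
; A timer re-arms itself at random intervals, spawning a Niagara bubble burst at the mouth socket and calling Play on the timeline again.
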(event `self.ReceiveBeginPlay`
  (bind _returnvalue (- 1.0 (`KismetMathLibrary.FClamp` (/ (`KismetMathLibrary.VSize` (`PrimitiveComponent.GetPhysicsAngularVelocityInDegrees` (`self.SkeletalMesh`) "None")) 4.0))))
  (`KismetSystemLibrary.K2_SetTimerDelegate` (delegate `CustomEvent`) (`KismetMathLibrary.RandomFloatInRange` 5.0 9.0) :!label _label)
  (bind (_direction _headtrack) (`Timeline|SwimmingTimeline`)
    (:`Update`
      (set `self.HeadLocation` (`KismetMathLibrary.MakeVector` (* (* _headtrack (/ (`KismetMathLibrary.VSize` (`self.GetVelocity`)) (`MovementComponent.GetMaxSpeed` (`self.FloatingPawnMovement`)))) 600.0)))
      (set `self.NormalizedElasticity` _returnvalue)
      (`KismetSystemLibrary.PrintString` (`KismetStringLibrary.Conv_DoubleToString` _returnvalue) true true (struct :`G` 0.66 :`B` 1.0 :`A` 1.0) 0.0))))

(event `CustomEvent`
  (`NiagaraFunctionLibrary.SpawnSystemAtLocation` "/Game/VFX/Particles/NS_BubbleBurst.NS_BubbleBurst" (`SceneComponent.GetSocketLocation` (`self.SkeletalMesh`) "Mouth") (struct) (2.0 2.0 2.0))
  (goto _label))

(event `self.ReceiveTick`
  (params (DeltaSeconds :type "Float (single-precision)")))

(fn `UserConstructionScript`)