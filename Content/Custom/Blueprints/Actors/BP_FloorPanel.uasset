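; BP_FloorPanel is an underwater floor tile that randomly dresses itself with kelp and bubbles on BeginPlay.
; Three kelp spots roll against Chance to spawn one of two tall kelp meshes, varied by random scale and Y-axis mirroring.
; Three bubble spots use a fixed chance to spawn a Niagara bubble effect with a random amount.
; GetNextTileLocation exposes the NextStartLocation world position for placing the following tile.
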(event `self.ReceiveBeginPlay`
  (`self.AddRandomKelp` (`self.KelpLocation_01`) (`self.Chance`))
  (`self.AddRandomKelp` (`self.KelpLocation_02`) (`self.Chance`))
  (`self.AddRandomKelp` (`self.KelpLocation_03`) (`self.Chance`))
  (`self.AddRandomBubble` (`self.bubbleLocation_02`) 0.25)
  (`self.AddRandomBubble` (`self.bubbleLocation_01`) 0.25)
  (`self.AddRandomBubble` (`self.bubbleLocation_03`) 0.25))

(fn `AddRandomBubble`
  (params (kelpSpot :type "SceneComponent Object Reference") (Chance :type "Float (double-precision)"))
  (if (>= Chance (`KismetMathLibrary.RandomFloat`))
    (bind _returnvalue (`AddComponent|NODE_AddNiagaraComponent-0` :`RelativeTransform` (`SceneComponent.GetRelativeTransform` kelpSpot)))
    (`NiagaraComponent.SetAsset` _returnvalue "/Game/VFX/Particles/NS_BubblesConstant.NS_BubblesConstant" true)
    (`NiagaraComponent.SetVariableFloat` _returnvalue "BubblesAmount" (`KismetMathLibrary.RandomFloatInRange` 0.2 1.2))))

(fn `AddRandomKelp`
  (params (kelpSpot :type "SceneComponent Object Reference") (Chance :type "Float (double-precision)"))
  (bind _returnvalue (`KismetMathLibrary.RandomFloatInRange` 0.9 1.1))
  (bind _returnvalue_2 (`KismetMathLibrary.MakeVector` _returnvalue _returnvalue _returnvalue))
  (if (>= Chance (`KismetMathLibrary.RandomFloat`))
    (bind _returnvalue_3 (`AddComponent|NODE_AddStaticMeshComponent-0` :`RelativeTransform` (`SceneComponent.GetRelativeTransform` kelpSpot)))
    (`|ExecutionSequence`
      (:`then_0`
        (if (> (`KismetMathLibrary.RandomFloat`) 0.5)
          (`StaticMeshComponent.SetStaticMesh` _returnvalue_3 "/Game/Custom/Meshes/tallkelp2.tallkelp2")
          (else
            (`StaticMeshComponent.SetStaticMesh` _returnvalue_3 "/Game/Custom/Meshes/tallkelp1.tallkelp1"))))
      (:`then_1`
        (if (> (`KismetMathLibrary.RandomFloat`) 0.5)
          (`SceneComponent.SetWorldScale3D` _returnvalue_3 (* _returnvalue_2 (`KismetMathLibrary.MakeVector` 1.0 -1.0 1.0)))
          (else
            (`SceneComponent.SetWorldScale3D` _returnvalue_3 _returnvalue_2)))))))

(fn `GetNextTileLocation`
  (returns (NextTileLocation :type "Vector Structure"))
  (return (`SceneComponent.K2_GetComponentLocation` (`self.NextStartLocation`))))

(fn `UserConstructionScript`)