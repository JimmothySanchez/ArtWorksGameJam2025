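; BP_Building_Honeycomb is a honeycomb building actor that animates its mesh into place when play begins.
; BeginPlay calls the parent, then plays a timeline that lerps the static mesh's relative Z from a high offset down to zero, assuming the track runs zero to one.
; The construction script only calls the parent, and the overlap and tick events are disabled stubs.
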(event `self.ReceiveBeginPlay`
  (`parent.ReceiveBeginPlay`)
  (bind (_direction _newtrack_0) (`Timeline|Timeline`)
    (:`Update`
      (`SceneComponent.K2_SetRelativeLocation` (`self.StaticMesh`) (`KismetMathLibrary.MakeVector` 0.0 0.0 (`KismetMathLibrary.Lerp` 2000.0 0.0 _newtrack_0)) false false))))

(fn `UserConstructionScript`
  (`parent.UserConstructionScript`))