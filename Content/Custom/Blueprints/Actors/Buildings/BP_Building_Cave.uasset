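; Cave building actor that stages its own arrival with Level Sequences when play begins.
; It hides its static mesh, plays the cave drop sequence, then reveals the mesh when that sequence finishes.
; In parallel, after a short delay, it plays a tentacle test sequence at the TentacleTransform component.
; Both sequences override instance data to set their transform origin, so they play relative to the placed building.
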(event `CustomEvent_0`
  (`SceneComponent.SetHiddenInGame` (`self.StaticMesh`) false false))

(event `self.ReceiveBeginPlay`
  (`parent.ReceiveBeginPlay`)
  (`|ExecutionSequence`
    (:`then_0`
      (`SceneComponent.SetHiddenInGame` (`self.StaticMesh`) true false)
      (bind _outactor (`LevelSequencePlayer.CreateLevelSequencePlayer` "/Game/Custom/Anims/LS_CaveDrop.LS_CaveDrop"))
      (set `LevelSequenceActor.bOverrideInstanceData` true _outactor)
      (bind _asdefault_level_sequence_instance_data (cast `DefaultLevelSequenceInstanceData` (`LevelSequenceActor.DefaultInstanceData` _outactor)))
      (set `DefaultLevelSequenceInstanceData.TransformOrigin` (`self.GetTransform`) _asdefault_level_sequence_instance_data)
      (bind _sequenceplayer (`LevelSequenceActor.SequencePlayer` _outactor))
      (add `MovieSceneSequencePlayer.OnFinished` _sequenceplayer (delegate `CustomEvent_0`))
      (`MovieSceneSequencePlayer.Play` _sequenceplayer))
    (:`then_1`
      (`KismetSystemLibrary.Delay` 4.0)
      (bind _outactor_2 (`LevelSequencePlayer.CreateLevelSequencePlayer` "/Game/Custom/Anims/Tentacle_Test.Tentacle_Test"))
      (set `LevelSequenceActor.bOverrideInstanceData` true _outactor_2)
      (bind _asdefault_level_sequence_instance_data_2 (cast `DefaultLevelSequenceInstanceData` (`LevelSequenceActor.DefaultInstanceData` _outactor_2)))
      (set `DefaultLevelSequenceInstanceData.TransformOrigin` (`SceneComponent.K2_GetComponentToWorld` (`self.Tentacle_Transform`)) _asdefault_level_sequence_instance_data_2)
      (`MovieSceneSequencePlayer.Play` (`LevelSequenceActor.SequencePlayer` _outactor_2)))))

(fn `UserConstructionScript`
  (`parent.UserConstructionScript`))