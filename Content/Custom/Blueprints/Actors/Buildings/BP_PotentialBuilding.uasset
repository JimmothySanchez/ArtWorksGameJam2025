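; Preview actor that stands in for a potential building, showing a given static mesh in a debug material.
; UpdateMesh swaps the mesh, then overrides every material slot with Mat_DebugPotentialBuilding.
; SetScale stores a uniform scale and applies it to the mesh component's relative scale, and GetScale returns the stored value.
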(fn `GetScale`
  (returns (Scale :type "Float (double-precision)"))
  (return (`self.Scale`)))

(fn `SetScale`
  (params (Scale :type "Float (double-precision)"))
  (bind _output_get (set `self.Scale` Scale))
  (`SceneComponent.SetRelativeScale3D` (`self.StaticMesh`) (`KismetMathLibrary.MakeVector` _output_get _output_get _output_get)))

(fn `UpdateMesh`
  (params (newMesh :type "StaticMesh Object Reference"))
  (bind _staticmesh (`self.StaticMesh`))
  (`StaticMeshComponent.SetStaticMesh` _staticmesh newMesh)
  (for _index (range (+ (`KismetArrayLibrary.Array_LastIndex` (`PrimitiveComponent.GetMaterialSlotNames` _staticmesh)) 1))
    (`PrimitiveComponent.SetMaterial` _staticmesh _index "/Game/Custom/Materials/Debug_Mats/Mat_DebugPotentialBuilding.Mat_DebugPotentialBuilding")))

(fn `UserConstructionScript`)