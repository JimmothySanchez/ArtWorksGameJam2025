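; BP_Building_FishFood is a fish food building actor that plays the FishFeedAnimation level sequence where it is placed.
; On BeginPlay it creates a sequence player, overrides the instance data's transform origin with its own transform so the animation plays relative to it, then starts playback.
; It destroys itself when the spawned sequence actor fires OnEndPlay, rather than binding to the player's finished event.
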(event `self.ReceiveBeginPlay`
  (`parent.ReceiveBeginPlay`)
  (bind _outactor (`LevelSequencePlayer.CreateLevelSequencePlayer` (`self.FishFeedAnimation`)))
  (set `LevelSequenceActor.bOverrideInstanceData` true _outactor)
  (bind _asdefault_level_sequence_instance_data (cast `DefaultLevelSequenceInstanceData` (`LevelSequenceActor.DefaultInstanceData` _outactor)))
  (set `DefaultLevelSequenceInstanceData.TransformOrigin` (`self.GetTransform`) _asdefault_level_sequence_instance_data)
  (add `self.OnEndPlay` _outactor (delegate `CustomEvent`))
  (`MovieSceneSequencePlayer.Play` (`LevelSequenceActor.SequencePlayer` _outactor)))

(event `CustomEvent` :!signature `self.OnEndPlay`
  (params (Actor :type "Actor Object Reference") (EndPlayReason :type "EEndPlayReason Enum" :default "Destroyed"))
  (`self.K2_DestroyActor`))

(fn `UserConstructionScript`
  (`parent.UserConstructionScript`))