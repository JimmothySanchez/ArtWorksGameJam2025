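; Coral rock building actor that plays the generic drop Level Sequence on itself at BeginPlay.
; It creates a sequence player for LS_GenericDrop and binds itself to the sequence at runtime.
; An instance-data override sets the transform origin to the actor's location and rotation at unit scale, so the shared animation plays relative to where the building stands.
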(event `self.ReceiveBeginPlay`
  (`parent.ReceiveBeginPlay`)
  (bind _outactor (`LevelSequencePlayer.CreateLevelSequencePlayer` "/Game/Custom/Anims/LS_GenericDrop.LS_GenericDrop"))
  (`LevelSequenceActor.AddBinding` _outactor (`|GetSequenceBinding` null) self false)
  (set `LevelSequenceActor.bOverrideInstanceData` true _outactor)
  (bind _asdefault_level_sequence_instance_data (cast `DefaultLevelSequenceInstanceData` (`LevelSequenceActor.DefaultInstanceData` _outactor)))
  (set `DefaultLevelSequenceInstanceData.TransformOrigin` (`KismetMathLibrary.MakeTransform` (.location (`self.GetTransform`)) (.rotation (`self.GetTransform`))) _asdefault_level_sequence_instance_data)
  (`MovieSceneSequencePlayer.Play` (`LevelSequenceActor.SequencePlayer` _outactor)))

(fn `UserConstructionScript`
  (`parent.UserConstructionScript`))