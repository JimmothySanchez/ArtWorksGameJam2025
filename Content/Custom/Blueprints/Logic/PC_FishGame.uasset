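; Player controller for the fish game that creates the HUD, shows the cursor, and handles pausing and mouse-driven building placement.
; Selecting a build type tags the controller as queued and spawns a hidden preview actor with randomized scale and optional random yaw.
; Each tick a cursor trace moves and shows the preview, which input can rotate.
; Building spawns the selected class with the preview's rotation and scale, then clears the selection.
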(event `self.ReceiveBeginPlay`
  (bind _returnvalue (`|CreateWidget` "/Game/Custom/UI/WDG_HUD.WDG_HUD_C"))
  (set `self.HUD` _returnvalue)
  (`UserWidget.AddToViewport` _returnvalue 0)
  (`WidgetBlueprintLibrary.SetInputMode_GameAndUIEx` self _returnvalue "DoNotLock" false)
  (set `self.bShowMouseCursor` true))

(event `self.ReceiveTick`
  (params (DeltaSeconds :type "Float (single-precision)"))
  (if (`BlueprintGameplayTagLibrary.HasTag` (`self.TagContainer`) (struct :`TagName` "Interaction.HasbuildingQueued"))
    (bind (_location _validhit) (`self.GetUnderMouseLocation`))
    (`self.DrawPotentialBuilding` _location _validhit)))

(event `EnhancedInput|/Game/Custom/Input/IA_Build`
  (params (ActionValue :type Boolean) (ElapsedSeconds :type "Float (double-precision)") (TriggeredSeconds :type "Float (double-precision)") (InputAction :type "InputAction Object Reference" :default "/Game/Custom/Input/IA_Build.IA_Build"))
  (:`Started`
    (bind (_location _validhit) (`self.GetUnderMouseLocation`))
    (if _validhit
      (`self.BuildBuilding` _location))))

(event `EnhancedInput|/Game/Custom/Input/IA_Pause`
  (params (ActionValue :type Boolean) (ElapsedSeconds :type "Float (double-precision)") (TriggeredSeconds :type "Float (double-precision)") (InputAction :type "InputAction Object Reference" :default "/Game/Custom/Input/IA_Pause.IA_Pause"))
  (:`Started`
    (bind _isa (`/Engine/EditorBlueprintResources/StandardMacros.FlipFlop`)
      (:`A`
        (`GameplayStatics.SetGamePaused` _isa))
      (:`B`
        (`GameplayStatics.SetGamePaused` false)))))

(event `EnhancedInput|/Game/Custom/Input/IA_RotateBuilding`
  (params (ActionValue :type "Float (double-precision)") (ElapsedSeconds :type "Float (double-precision)") (TriggeredSeconds :type "Float (double-precision)") (InputAction :type "InputAction Object Reference" :default "/Game/Custom/Input/IA_RotateBuilding.IA_RotateBuilding"))
  (:`Triggered`
    (if (`BlueprintGameplayTagLibrary.HasTag` (`self.TagContainer`) (struct :`TagName` "Interaction.HasbuildingQueued"))
      (`self.K2_AddActorWorldRotation` (`self.PotentialBuilding`) (`KismetMathLibrary.MakeRotator` 0.0 0.0 (* ActionValue (`self.RotationMultiplier`))) false false))))

(fn `BuildBuilding`
  (params (location :type "Vector Structure"))
  (bind _potentialbuilding (`self.PotentialBuilding`))
  (bind _scale (`/Game/Custom/Blueprints/Actors/Buildings/BP_PotentialBuilding.GetScale` _potentialbuilding))
  (`/Engine/EditorBlueprintResources/StandardMacros.IsValid` _potentialbuilding
    (:`Is Valid`
      (`|SpawnActorFromClass` (`self.SelectedBuilding`) (`KismetMathLibrary.MakeTransform` location (`self.K2_GetActorRotation` _potentialbuilding) (`KismetMathLibrary.MakeVector` _scale _scale _scale)) "Undefined" "MultiplyWithRoot" null null)
      (`self.ClearBuildType`))))

(fn `ClearBuildType`
  (bind _potentialbuilding (`self.PotentialBuilding`))
  (set `self.SelectedBuilding` null)
  (`BlueprintGameplayTagLibrary.RemoveGameplayTag` (`self.TagContainer`) (struct :`TagName` "Interaction.HasbuildingQueued"))
  (`/Engine/EditorBlueprintResources/StandardMacros.IsValid` _potentialbuilding
    (:`Is Valid`
      (`self.K2_DestroyActor` _potentialbuilding))))

(fn `DrawPotentialBuilding`
  (params (Location :type "Vector Structure") (IsValid :type Boolean))
  (`SceneComponent.SetVisibility` (`/Game/Custom/Blueprints/Actors/Buildings/BP_PotentialBuilding.StaticMesh` (`self.PotentialBuilding`)) IsValid false)
  (`self.K2_SetActorLocation` (`self.PotentialBuilding`) Location false false))

(fn `GetUnderMouseLocation`
  (returns (Location :type "Vector Structure") (ValidHit :type Boolean))
  (bind (_worldlocation _worlddirection) (`self.DeprojectMousePositionToWorld`))
  (bind (_outhit _returnvalue) (`KismetSystemLibrary.LineTraceSingle` :`Start` _worldlocation :`End` (+ _worldlocation (* _worlddirection (`self.TraceDistance`))) :`TraceChannel` "TraceTypeQuery1" :`bTraceComplex` true :`DrawTime` 3.0))
  (return (`.Location` (`GameplayStatics.BreakHitResult` _outhit)) _returnvalue))

(fn `SetBuildType`
  (params (BuildingType :type "/Game/Custom/Data/PDA_BuildingType Object Reference"))
  (`|ExecutionSequence`
    (:`then_0`
      (`/Engine/EditorBlueprintResources/StandardMacros.IsValid` (`self.PotentialBuilding`)
        (:`Is Valid`
          (`self.K2_DestroyActor` (`self.PotentialBuilding`)))))
    (:`then_1`
      ; Set type
      (set `self.SelectedBuilding` (`/Game/Custom/Data/PDA_BuildingType.Building` BuildingType))
      (`BlueprintGameplayTagLibrary.AddGameplayTag` (`self.TagContainer`) (struct :`TagName` "Interaction.HasbuildingQueued"))
      (bind _returnvalue (`|SpawnActorFromClass` "/Game/Custom/Blueprints/Actors/Buildings/BP_PotentialBuilding.BP_PotentialBuilding_C" (`KismetMathLibrary.MakeTransform` (0.0 0.0 0.0)) "Undefined" "MultiplyWithRoot" null null))
      (set `self.PotentialBuilding` _returnvalue)
      (`/Game/Custom/Blueprints/Actors/Buildings/BP_PotentialBuilding.UpdateMesh` _returnvalue (`/Game/Custom/Data/PDA_BuildingType.PreviewMesh` BuildingType))
      (`SceneComponent.SetVisibility` (`/Game/Custom/Blueprints/Actors/Buildings/BP_PotentialBuilding.StaticMesh` _returnvalue) false false))
    (:`then_2`
      ; Scale
      (`/Game/Custom/Blueprints/Actors/Buildings/BP_PotentialBuilding.SetScale` (`self.PotentialBuilding`) (`KismetMathLibrary.RandomFloatInRange` (`/Game/Custom/Data/PDA_BuildingType.MinScale` BuildingType) (`/Game/Custom/Data/PDA_BuildingType.MaxScale` BuildingType))))
    (:`then_3`
      (if (`/Game/Custom/Data/PDA_BuildingType.RandomInitialRot` BuildingType)
        (`self.K2_SetActorRotation` (`self.PotentialBuilding`) (`KismetMathLibrary.MakeRotator` 0.0 0.0 (`KismetMathLibrary.RandomFloatInRange` 0.0 360.0)) false)))))

(fn `UserConstructionScript`)