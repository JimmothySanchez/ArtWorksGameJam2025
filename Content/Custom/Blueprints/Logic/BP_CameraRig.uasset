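; Player camera rig for the fish game, toggling overhead and side views (HUD hidden in side view) and taking screenshots.
; Opens a borderless second-monitor window and resizes its render target to match.
; Trigger volumes spawn floor panels as tiles exit and destroy actors not tagged SelfRecycling.
; Each tick, building count drives Niagara fish spawn rate and spawns one hero eel, always at SpawnLocation02 because RandomFloat never exceeds 5.
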(event `self.ReceiveBeginPlay`
  (bind _returnvalue (subsystem `MultiWindowExtensionSubsystem`))
  (bind _asplayer_controller (cast `PlayerController` (`self.GetController`)))
  (`EnhancedInputSubsystemInterface.AddMappingContext` (pcsubsystem `EnhancedInputLocalPlayerSubsystem` _asplayer_controller) "/Game/Custom/Input/IMC_FishGame.IMC_FishGame" 0 (struct))
  (`self.CameraSet` "NewEnumerator0")
  (`MultiWindowExtensionSubsystem.KB_MWE_Create` _returnvalue "/Game/Custom/UI/WDG_SecondWindow.WDG_SecondWindow_C" (make `KB_MWE_WindowSettings` "My Newly Created Window" (1000.0 1000.0) 2 "CenteredOnScreen" (0.0 0.0) "Borderless" "Maximized" 1.0 1.0 "UserSized" (struct :`A` 1.0) (struct :`UserResizeBorderMargin` (struct :`Left` 3.0 :`Top` 3.0 :`Right` 3.0 :`Bottom` 3.0)) (make `KB_MWE_WindowSizeRestrictionSettings` false)))
  (add `MultiWindowExtensionSubsystem.OnSizeChanged` _returnvalue (delegate `CustomEvent`)))

(event `CustomEvent`
  (params (WindowName :type String) (WindowID :type Integer64) (NewSize :type "Vector2D Structure"))
  (bind (_x _y) (`KismetMathLibrary.BreakVector2D` NewSize))
  (bind _returnvalue (`KismetMathLibrary.FTrunc` _x))
  (bind _returnvalue_2 (`KismetMathLibrary.FTrunc` _y))
  (`KismetRenderingLibrary.ResizeRenderTarget2D` "/Game/Custom/Materials/RT_SecondWindow.RT_SecondWindow" _returnvalue _returnvalue_2)
  (`KismetSystemLibrary.PrintText` (`|FormatText` "New size {x} x {y}" _returnvalue _returnvalue_2)))

(event `self.ReceiveTick`
  (params (DeltaSeconds :type "Float (single-precision)"))
  (`self.UpdateFish`))

(event `self.Recycler.OnComponentBeginOverlap`
  (params (OverlappedComponent :type "PrimitiveComponent Object Reference") (OtherActor :type "Actor Object Reference") (OtherComp :type "PrimitiveComponent Object Reference") (OtherBodyIndex :type Integer) (bFromSweep :type Boolean) (SweepResult :type "HitResult Structure (by ref)")))

(event `self.Recycler.OnComponentEndOverlap`
  (params (OverlappedComponent :type "PrimitiveComponent Object Reference") (OtherActor :type "Actor Object Reference") (OtherComp :type "PrimitiveComponent Object Reference") (OtherBodyIndex :type Integer))
  (if (not (`self.ActorHasTag` OtherActor "SelfRecycling"))
    (`self.K2_DestroyActor` OtherActor)))

(event `self.FloorTileCreator.OnComponentEndOverlap`
  (params (OverlappedComponent :type "PrimitiveComponent Object Reference") (OtherActor :type "Actor Object Reference") (OtherComp :type "PrimitiveComponent Object Reference") (OtherBodyIndex :type Integer))
  (if (`KismetSystemLibrary.DoesImplementInterface` OtherActor "/Game/Custom/Blueprints/Logic/BPI_Tile.BPI_Tile_C")
    (bind _nexttilelocation (message `/Game/Custom/Blueprints/Logic/BPI_Tile.GetNextTileLocation` OtherActor))
    (`|SpawnActorFromClass` "/Game/Custom/Blueprints/Actors/BP_FloorPanel.BP_FloorPanel_C" (`KismetMathLibrary.MakeTransform` _nexttilelocation) "Undefined" "MultiplyWithRoot" null null)))

(event `EnhancedInput|/Game/Custom/Input/IA_ScreenShot`
  (params (ActionValue :type Boolean) (ElapsedSeconds :type "Float (double-precision)") (TriggeredSeconds :type "Float (double-precision)") (InputAction :type "InputAction Object Reference" :default "/Game/Custom/Input/IA_ScreenShot.IA_ScreenShot"))
  (:`Started`
    (`AutomationBlueprintFunctionLibrary.TakeHighResScreenshot` 0 0 "" null)))

(event `EnhancedInput|/Game/Custom/Input/IA_CameraSwitch`
  (params (ActionValue :type Boolean) (ElapsedSeconds :type "Float (double-precision)") (TriggeredSeconds :type "Float (double-precision)") (InputAction :type "InputAction Object Reference" :default "/Game/Custom/Input/IA_CameraSwitch.IA_CameraSwitch"))
  (:`Started`
    (`self.CameraSwitch`)))

(fn `CameraSet`
  (params (Angle :type "/Game/Custom/Blueprints/Logic/En_CameraAngles Enum" :default "NewEnumerator0"))
  (bind _output_get (set `self.CurrentView` Angle))
  (switch `/Game/Custom/Blueprints/Logic/En_CameraAngles` _output_get
    (:`NewEnumerator0`
      (`ActorComponent.SetActive` (`self.SideviewCamera`) false false)
      (`ActorComponent.SetActive` (`self.OverheadCamera`) true false))
    (:`NewEnumerator1`
      (`ActorComponent.SetActive` (`self.OverheadCamera`) false false)
      (`ActorComponent.SetActive` (`self.SideviewCamera`) true false))))

(fn `CameraSwitch`
  (bind _aspc_fish_game (cast `/Game/Custom/Blueprints/Logic/PC_FishGame` (`self.GetController`)))
  (switch `/Game/Custom/Blueprints/Logic/En_CameraAngles` (`self.CurrentView`)
    (:`NewEnumerator0`
      (`self.CameraSet` "NewEnumerator1")
      (bind _hud (`/Game/Custom/Blueprints/Logic/PC_FishGame.HUD` _aspc_fish_game))
      (set `Widget.Visibility` "Hidden" _hud))
    (:`NewEnumerator1`
      (`self.CameraSet` "NewEnumerator0")
      (set `Widget.Visibility` "Visible" _hud))))

(fn `GetRandomSpawnLocation`
  (returns (NewParam :type "Vector Structure"))
  (if (> (`KismetMathLibrary.RandomFloat`) 5.0)
    (return (`SceneComponent.K2_GetComponentLocation` (`self.SpawnLocation_01`)))
    (else
      (return (`SceneComponent.K2_GetComponentLocation` (`self.SpawnLocation_02`))))))

(fn `UpdateFish`
  (locals (BuildingCount :type Integer :default 0))
  (`|ExecutionSequence`
    (:`then_0`
      ; UpdateCount
      (bind _outactors (`GameplayStatics.GetAllActorsOfClass` "/Game/Custom/Blueprints/Actors/Buildings/BP_BuildingBase.BP_BuildingBase_C"))
      (set `local.BuildingCount` (`KismetArrayLibrary.Array_Length` _outactors)))
    (:`then_1`
      ; Update Niagara
      (`NiagaraComponent.SetVariableFloat` (`self.FishSystem`) "FishSpawnRate" (`KismetMathLibrary.FClamp` (* (`local.BuildingCount`) 0.1) 0.1 5.0)))
    (:`then_2`
      ; Spawn a Hero Fish
      (bind _outactors_2 (`GameplayStatics.GetAllActorsOfClass` "/Game/Custom/Blueprints/Actors/Eel/BP_Eel.BP_Eel_C"))
      (if (and (> (`local.BuildingCount`) 5) (<= (`KismetArrayLibrary.Array_Length` _outactors_2) 0))
        (`|SpawnActorFromClass` "/Game/Custom/Blueprints/Actors/Eel/BP_Eel.BP_Eel_C" (`KismetMathLibrary.MakeTransform` (`self.GetRandomSpawnLocation`)) "AdjustIfPossibleButAlwaysSpawn" "MultiplyWithRoot" null null)
        (`KismetSystemLibrary.PrintString` "eel")))))

(fn `UserConstructionScript`)