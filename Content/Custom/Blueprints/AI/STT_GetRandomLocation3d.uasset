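; StateTree task that picks a random 3D location around the owning pawn, at roughly Radius give or take RadiusOffset.
; On state entry it loops, offsetting from the pawn along random directions and forcing Z positive with a small lift.
; A complex visibility trace back to the pawn rejects blocked candidates.
; After more than ten failures it falls back to a fixed X-axis offset from the pawn, and always finishes successfully.
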(event `self.ReceiveLatentEnterState`
  (params (Transition :type "StateTreeTransitionResult Structure (by ref)"))
  (bind _returnvalue (`Actor.K2_GetActorLocation` (`self.OwningPawn`)))
  (set `self.FailureCount` 0)
  (set `self.LocationIsValid` false)
  (while (not (`self.LocationIsValid`))
    (bind _output_get (set `self.RandomLocation` (`KismetMathLibrary.MakeVector` (.x (+ _returnvalue (* (`KismetMathLibrary.RandomUnitVector`) (`KismetMathLibrary.RandomFloatInRange` (- (`self.Radius`) (`self.RadiusOffset`)) (+ (`self.RadiusOffset`) (`self.Radius`)))))) (.y (+ _returnvalue (* (`KismetMathLibrary.RandomUnitVector`) (`KismetMathLibrary.RandomFloatInRange` (- (`self.Radius`) (`self.RadiusOffset`)) (+ (`self.RadiusOffset`) (`self.Radius`)))))) (+ (`KismetMathLibrary.Abs` (.z (+ _returnvalue (* (`KismetMathLibrary.RandomUnitVector`) (`KismetMathLibrary.RandomFloatInRange` (- (`self.Radius`) (`self.RadiusOffset`)) (+ (`self.RadiusOffset`) (`self.Radius`))))))) 100.0))))
    (bind (_outhits _returnvalue_2) (`KismetSystemLibrary.LineTraceMulti` _output_get _returnvalue "TraceTypeQuery1" true (`|MakeArray` (`self.OwningPawn`)) "None" true (struct :`R` 1.0 :`A` 1.0) (struct :`G` 1.0 :`A` 1.0) 2.0))
    (if _returnvalue_2
      (`/Engine/EditorBlueprintResources/StandardMacros.IncrementInt` (`self.FailureCount`)
        (:`  `
          (if (> (`self.FailureCount`) 10)
            ; handle path issue
            (set `self.RandomLocation` (+ (`Actor.K2_GetActorLocation` (`self.OwningPawn`)) (-8000.0 0.0 0.0)))
            (set `self.LocationIsValid` true))))
      (else
        (set `self.LocationIsValid` true))))
  (`self.FinishTask` true))