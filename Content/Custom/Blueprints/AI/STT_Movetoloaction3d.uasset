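; StateTree task that moves the owning pawn through 3D space toward a Location until it is closer than MinimumDistance.
; Each tick it feeds the direction to the target into the pawn's FloatingPawnMovement as straight-line steering, with no pathfinding.
; It also blends the pawn's rotation halfway toward the target every tick, independent of delta time, and finishes successfully once within range.
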(event `self.ReceiveLatentEnterState`
  (params (Transition :type "StateTreeTransitionResult Structure (by ref)")))

(event `self.ReceiveLatentTick`
  (params (DeltaTime :type "Float (single-precision)"))
  (bind _returnvalue (`KismetMathLibrary.FindLookAtRotation` (`Actor.K2_GetActorLocation` (`self.OwningPawn`)) (`self.Location`)))
  (`PawnMovementComponent.AddInputVector` (`Actor.GetComponentByClass` (`self.OwningPawn`) "/Script/Engine.FloatingPawnMovement") (`KismetMathLibrary.GetForwardVector` _returnvalue) false)
  (`Actor.K2_SetActorRotation` (`self.OwningPawn`) (`KismetMathLibrary.RLerp` (`Actor.K2_GetActorRotation` (`self.OwningPawn`)) _returnvalue 0.5 true) false)
  (if (< (`KismetMathLibrary.Vector_Distance` (`Actor.K2_GetActorLocation` (`self.OwningPawn`)) (`self.Location`)) (`self.MinimumDistance`))
    (`self.FinishTask` true)))