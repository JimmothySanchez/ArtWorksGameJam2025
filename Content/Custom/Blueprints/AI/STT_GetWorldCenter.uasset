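; StateTree task that supplies the location of the world center as its output.
; On entering the state, it takes the first actor tagged "WorldCenter", writes its location to OutLocation and finishes successfully, with no check for a missing actor.
; An unconnected leftover graph picks random points in a radius band around the owning pawn until a visibility trace back is clear, with debug drawing.
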(event `self.ReceiveLatentEnterState`
  (params (Transition :type "StateTreeTransitionResult Structure (by ref)"))
  (bind _outactors (`GameplayStatics.GetAllActorsWithTag` "WorldCenter"))
  (set `self.OutLocation` (`Actor.K2_GetActorLocation` (`|GetArrayItem` _outactors)))
  (`self.FinishTask` true))